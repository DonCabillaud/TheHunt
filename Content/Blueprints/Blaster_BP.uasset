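; Blaster weapon Blueprint whose Fire function spawns laser projectiles from the SpawnBullet point according to the current ShootMode.
; A visibility trace from the player Hunter's follow camera finds the aim point, using the hit or the trace end, and projectiles rotate toward it.
; Modes cover a normal laser, a shotgun burst with random pitch and yaw spread scaled by Precision, and a bouncing laser.
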(fn ConstructionScript)

(fn Fire
  (bind _spawnbullet (Variables|Default|GetspawnBullet))
  (bind _precision (Variables|Default|Getprecision))
  (bind _returnvalue (Transformation|GetWorldTransform _spawnbullet))
  ;[1 1 1] Orientation des projectiles
  (bind _ashunter_bp (Utilities|Casting|CastToHunter_BP (Game|GetPlayerCharacter 0)))
  (bind _outhit (Collision|LineTraceByChannel (Transformation|GetWorldLocation (Variables|/Game/Blueprints/Hunter_BP.Hunter_BP_C|GetFollowCamera _ashunter_bp)) (+ (Transformation|GetWorldLocation (Variables|/Game/Blueprints/Hunter_BP.Hunter_BP_C|GetFollowCamera _ashunter_bp)) (* (Math|Vector|GetForwardVector (Transformation|GetWorldRotation (Variables|/Game/Blueprints/Hunter_BP.Hunter_BP_C|GetFollowCamera _ashunter_bp))) 2.5e+03)) "TraceTypeQuery1" false 0 "None"))
  ;[1 1 1] Normal Shot
  (if (== (Variables|Default|GetshootMode) 0)
    (Game|SpawnActorfromClass "/Game/FX/LaserTrack/RedLaserTrack/BP_NormalLaser.BP_NormalLaser_C" (Math|Transform|MakeTransform (.location _returnvalue) (Math|Rotator|FindLookatRotation (.location _returnvalue) (Math|Vector|SelectVector (.ImpactPoint (Collision|BreakHitResult _outhit)) (.TraceEnd (Collision|BreakHitResult _outhit)) (.bBlockingHit (Collision|BreakHitResult _outhit)))) "3.000000,3.000000,3.000000") "Undefined" 0 0)
    (else
      ;[1 1 1] ShotGun shot
      (if (== (Variables|Default|GetshootMode) 1)
        (for _index (range 0 (Variables|Default|GetnbShotGunProjectile))
          (Game|SpawnActorfromClass "/Game/FX/LaserTrack/RedLaserTrack/BP_ShotGunLaser.BP_ShotGunLaser_C" (Math|Transform|MakeTransform (.location _returnvalue) (Math|Rotator|MakeRotator (.Roll (Math|Rotator|BreakRotator (Math|Rotator|FindLookatRotation (.location _returnvalue) (Math|Vector|SelectVector (.ImpactPoint (Collision|BreakHitResult _outhit)) (.TraceEnd (Collision|BreakHitResult _outhit)) (.bBlockingHit (Collision|BreakHitResult _outhit)))))) (+ (* (- (Math|Random|RandomFloat) 0.5) _precision) (.Pitch (Math|Rotator|BreakRotator (Math|Rotator|FindLookatRotation (.location _returnvalue) (Math|Vector|SelectVector (.ImpactPoint (Collision|BreakHitResult _outhit)) (.TraceEnd (Collision|BreakHitResult _outhit)) (.bBlockingHit (Collision|BreakHitResult _outhit))))))) (+ (.Yaw (Math|Rotator|BreakRotator (Math|Rotator|FindLookatRotation (.location _returnvalue) (Math|Vector|SelectVector (.ImpactPoint (Collision|BreakHitResult _outhit)) (.TraceEnd (Collision|BreakHitResult _outhit)) (.bBlockingHit (Collision|BreakHitResult _outhit)))))) (* (- (Math|Random|RandomFloat) 0.5) _precision))) "3.000000,3.000000,3.000000") "Undefined" 0 0))
        (else
          ;[1 1 1] Boucing shot
          (if (== (Variables|Default|GetshootMode) 2)
            (Game|SpawnActorfromClass "/Game/FX/LaserTrack/RedLaserTrack/BP_BouncingLaserr.BP_BouncingLaserr_C" (Math|Transform|MakeTransform (.location _returnvalue) (Math|Rotator|FindLookatRotation (.location _returnvalue) (Math|Vector|SelectVector (.ImpactPoint (Collision|BreakHitResult _outhit)) (.TraceEnd (Collision|BreakHitResult _outhit)) (.bBlockingHit (Collision|BreakHitResult _outhit)))) "0.100000,0.100000,0.100000") "Undefined" 0 0)))))))