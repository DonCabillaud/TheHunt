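; Bridge actor that swaps a placeholder TobeBridge component for the finished Bridge when hit, despite its FallingMesh2 name.
; At BeginPlay it shows TobeBridge and hides Bridge.
; TobeBridge's hit event runs chained casts for shotgun, bouncing and normal lasers, then destroys TobeBridge and reveals Bridge.
; The swap uses only visibility and component destruction, with no movement or physics logic.
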(event OnComponentHit(TobeBridge)
  (params (HitComponent :type Primitive%20Component%20Object%20Reference) (OtherActor :type Actor%20Object%20Reference) (OtherComp :type Primitive%20Component%20Object%20Reference) (NormalImpulse :type Vector :default "0, 0, 0") (Hit :type Hit%20Result%20Structure%20%28by%20ref%29))
  (Utilities|Casting|CastToBP_ShotGunLaser OtherActor
    (:then
      _)
    (:CastFailed
      (Utilities|Casting|CastToBP_BouncingLaserr OtherActor
        (:then
          _)
        (:CastFailed
          (Utilities|Casting|CastToBP_NormalLaser OtherActor
            (:then
              _)
            (:CastFailed
              _))))))
  (Components|DestroyComponent (Variables|Default|GetTobeBridge))
  (Rendering|SetVisibility (Variables|Default|GetBridge) true false))

(event EventBeginPlay
  (Rendering|SetVisibility (Variables|Default|GetTobeBridge) true false)
  (Rendering|SetVisibility (Variables|Default|GetBridge) false false))

(event Collision|EventActorBeginOverlap
  (params (OtherActor :type Actor%20Object%20Reference)))

(event EventTick
  (params (DeltaSeconds :type Float%20%28single-precision%29)))

(fn ConstructionScript)