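; Foot IK component that computes foot and pelvis height offsets for the Hunter character, presumably for its animation to use.
; Each tick, TraceFromFoot line-traces down at a foot bone's XY from actor height to below the capsule, measuring ground offset.
; The left offset interpolates toward its trace, and the pelvis toward the larger foot offset.
; The right trace result is unused, as that interpolation targets RightFootOffset itself.
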(event EventBeginPlay)

(event EventTick
  (params (DeltaSeconds :type Float%20%28single-precision%29))
  (Variables|Default|SetDeltaSeconds DeltaSeconds)
  (bind _returnvalue (CallFunction|TracefromFoot (Variables|Parameter|GetLeftFootName) (Variables|Parameter|GetTraceDistBelowCapsule)))
  (Variables|Default|SetLeftFootOffset (Math|Interpolation|FInterpTo (Variables|Default|GetLeftFootOffset) _returnvalue (Variables|Default|GetDeltaSeconds) (Variables|Parameter|GetInterpSpeed)))
  (CallFunction|TracefromFoot (Variables|Parameter|GetRightFootName) (Variables|Parameter|GetTraceDistBelowCapsule))
  (Variables|Default|SetRightFootOffset (Math|Interpolation|FInterpTo 0.0 (Variables|Default|GetRightFootOffset) (Variables|Default|GetDeltaSeconds) (Variables|Parameter|GetInterpSpeed)))
  (Variables|Default|SetPelvisOffset (Math|Interpolation|FInterpTo (Variables|Default|GetPelvisOffset) (Math|Float|Max(Float) (Variables|Default|GetLeftFootOffset) (Variables|Default|GetRightFootOffset)) (Variables|Default|GetDeltaSeconds) (Variables|Parameter|GetInterpSpeed))))

(fn TracefromFoot
  (params (BoneName :type Name) (TraceDistBelowCapsule :type Float%20%28single-precision%29))
  (LocalVariables|SetL_TraceDisBelowCapsule TraceDistBelowCapsule)
  (LocalVariables|SetL_BoneLocation (Transformation|GetSocketLocation (Variables|/Script/Engine.Character|GetMesh (Variables|Default|GetHunter)) BoneName))
  (LocalVariables|SetL_TraceStartLocation (Math|Vector|MakeVector (.x (LocalVariables|GetL_BoneLocation)) (.y (LocalVariables|GetL_BoneLocation)) (.z (Transformation|GetActorLocation (Variables|Default|GetHunter)))))
  (LocalVariables|SetL_TraceEndLocation (Math|Vector|MakeVector (.x (LocalVariables|GetL_BoneLocation)) (.y (LocalVariables|GetL_BoneLocation)) (- (.z (Transformation|GetActorLocation (Variables|Default|GetHunter))) (+ (Components|Capsule|GetScaledCapsuleHalfHeight (Variables|/Script/Engine.Character|GetCapsuleComponent (Variables|Default|GetHunter))) (LocalVariables|GetL_TraceDisBelowCapsule)))))
  (bind (_outhit _returnvalue) (Collision|LineTraceByChannel (LocalVariables|GetL_TraceStartLocation) (LocalVariables|GetL_TraceEndLocation) "TraceTypeQuery2" true 0 "None"))
  (return (Math|Float|SelectFloat (- (Math|Vector|VectorLength (- (LocalVariables|GetL_TraceStartLocation) (.Location (Collision|BreakHitResult _outhit)))) (Components|Capsule|GetScaledCapsuleHalfHeight (Variables|/Script/Engine.Character|GetCapsuleComponent (Variables|Default|GetHunter)))) 0.0 _returnvalue)))