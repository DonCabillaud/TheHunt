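; BP_EnnemiLaser is an enemy laser projectile that damages Hunter_BP on hit.
; Each Tick stretches the PLaser beam between BulletCollision and Scene, and destroys the actor if X velocity is zero.
; Hits ignore Blaster_BP and BP_NormalLaser; other hits destroy it, as does a lifetime delay from BeginPlay.
; NormalDamage20, not called here, subtracts fixed Health from the first BombEnemy found.
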(event OnComponentHit(BulletCollision)
  (params (HitComponent :type Primitive%20Component%20Object%20Reference) (OtherActor :type Actor%20Object%20Reference) (OtherComp :type Primitive%20Component%20Object%20Reference) (NormalImpulse :type Vector :default "0, 0, 0") (Hit :type Hit%20Result%20Structure%20%28by%20ref%29))
  (Utilities|Casting|CastToBlaster_BP OtherActor
    (:CastFailed
      (Utilities|Casting|CastToBP_NormalLaser OtherActor
        (:CastFailed
          (bind _ashunter_bp (Utilities|Casting|CastToHunter_BP OtherActor)
            (:then
              (Default|DamageTaken _ashunter_bp (Variables|Default|Getdamage)))
            (:CastFailed
              _))
          (Actor|DestroyActor))))))

(event EventBeginPlay
  (Utilities|FlowControl|Delay 1e+01)
  (Actor|DestroyActor))

(event EventTick
  (params (DeltaSeconds :type Float%20%28single-precision%29))
  (Class|ParticleSystemComponent|SetBeamSourcePoint (Variables|Default|GetP_Laser) 0 (Transformation|GetWorldLocation (Variables|Default|GetBulletCollision)))
  (Class|ParticleSystemComponent|SetBeamEndPoint (Variables|Default|GetP_Laser) 0 (Transformation|GetWorldLocation (Variables|Default|GetScene)))
  (if (== (.x (Variables|/Script/Engine.MovementComponent|GetVelocity (Variables|Default|GetProjectileMovement))) 0.0)
    (Actor|DestroyActor)))

(fn ConstructionScript)

(fn NormalDamage20
  (bind _outactors (Actor|GetAllActorsOfClass "/Game/Blueprints/AI/BombEnemy.BombEnemy_C"))
  (Variables|/Game/Blueprints/AI/BombEnemy.BombEnemy_C|SetHealth (Utilities|Array|Get(acopy) _outactors) (- (Variables|/Game/Blueprints/AI/BombEnemy.BombEnemy_C|GetHealth (Utilities|Array|Get(acopy) _outactors)) 1.5e+02)))