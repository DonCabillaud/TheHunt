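; Test bouncing laser projectile that records its start and each hit point during a 0.1-second lifetime.
; Hits destroy DestroyEnvionment actors, and it ends early on enemies or the bounce limit.
; When destroyed, it draws the path as debug line traces between recorded points.
; HitFunction, uncalled here, scales enemy damage by bounces and aiming and grants the Hunter bullet time; NormalDamage20 is also uncalled.
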(event OnComponentHit(BulletCollision)
  (params (HitComponent :type Primitive%20Component%20Object%20Reference) (OtherActor :type Actor%20Object%20Reference) (OtherComp :type Primitive%20Component%20Object%20Reference) (NormalImpulse :type Vector :default "0, 0, 0") (Hit :type Hit%20Result%20Structure%20%28by%20ref%29))
  (bind _currentboucing (Variables|Default|GetcurrentBoucing))
  (Utilities|Array|Add (Variables|Default|Gethit%20point) (Transformation|GetWorldLocation (Variables|Default|GetBulletCollision)))
  (Utilities|Casting|CastToBlaster_BP OtherActor
    (:CastFailed
      (Utilities|Casting|CastToBP_BouncingLaserr OtherActor
        (:CastFailed
          (bind _asdestroy_envionment (Utilities|Casting|CastToDestroyEnvionment OtherActor)
            (:then
              (Actor|DestroyActor _asdestroy_envionment))
            (:CastFailed
              _))
          (Utilities|FlowControl|Sequence
            (:then_0
              (Utilities|Casting|CastToBombEnemy OtherActor
                (:then
                  _)
                (:CastFailed
                  (Utilities|Casting|CastToDistantEnemy OtherActor)))
              (Actor|DestroyActor :!label _label))
            (:then_1
              (if (== _currentboucing (Variables|Default|GetmaxBoucing))
                (goto _label)
                (else
                  (Math|Integer|IncrementInt _currentboucing))))))))))

(event EventBeginPlay
  (Utilities|Array|Add (Variables|Default|Gethit%20point) (Transformation|GetWorldLocation (Variables|Default|GetBulletCollision)))
  (Variables|Default|SetcurrentBoucing 0)
  (Utilities|FlowControl|Delay 0.1)
  (Actor|DestroyActor))

(event EventDestroyed
  (bind _hit_point (Variables|Default|Gethit%20point))
  (for _index (range 0 (- (Utilities|Array|LastIndex _hit_point) 1))
    (Collision|LineTraceByChannel (Utilities|Array|Get(acopy) _hit_point _index) (Utilities|Array|Get(acopy) _hit_point (+ _index 1)) "TraceTypeQuery1" false 0 "ForOneFrame" true "(R=0.000000,G=0.058824,B=1.000000,A=1.000000)" "(R=0.000000,G=0.058824,B=1.000000,A=1.000000)")))

(fn ConstructionScript)

(fn NormalDamage20
  (bind _outactors (Actor|GetAllActorsOfClass "/Game/Blueprints/AI/BombEnemy.BombEnemy_C"))
  (Variables|/Game/Blueprints/AI/BombEnemy.BombEnemy_C|SetHealth (Utilities|Array|Get(acopy) _outactors) (- (Variables|/Game/Blueprints/AI/BombEnemy.BombEnemy_C|GetHealth (Utilities|Array|Get(acopy) _outactors)) 1.5e+02)))

(fn HitFunction
  (params (distantEnnemis :type Distant%20Enemy%20Object%20Reference) (bombEnnemis :type Bomb%20Enemy%20Object%20Reference))
  (bind _ashunter_bp (Utilities|Casting|CastToHunter_BP (Game|Player|GetPlayerPawn 0)))
  (if (Variables|/Game/Blueprints/Hunter_BP.Hunter_BP_C|GetBulletTime _ashunter_bp)
    _
    (else
      (Default|BulletTimeGain _ashunter_bp (+ (Variables|Default|GetBulletTimePoint) (Math|Conversions|ToFloat(Integer) (Variables|Default|GetcurrentBoucing))))))
  (LocalVariables|SetdamageTaken (+ (Variables|Default|GetDamage) (* (Variables|Default|GetcurrentBoucing) (Variables|Default|GetdamageAdd))))
  (if (Utilities|IsValid distantEnnemis)
    (if (Variables|/Game/Blueprints/Hunter_BP.Hunter_BP_C|GetIsAiming _ashunter_bp)
      (Default|DamageTaken distantEnnemis (+ (LocalVariables|GetdamageTaken) 5.0))
      (else
        (Default|DamageTaken distantEnnemis (LocalVariables|GetdamageTaken))))
    (elif (Utilities|IsValid bombEnnemis)
      (if (Variables|/Game/Blueprints/Hunter_BP.Hunter_BP_C|GetIsAiming _ashunter_bp)
        (Default|DamageTaken bombEnnemis (+ (LocalVariables|GetdamageTaken) 5.0))
        (else
          (Default|DamageTaken bombEnnemis (LocalVariables|GetdamageTaken)))))))