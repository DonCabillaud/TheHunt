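; BP_ShotGunLaser is a shotgun laser projectile that damages bomb and distant enemies and destroys destructible environment actors.
; Tick stretches a beam particle between its collision and scene components, and it expires after travelling its maximum range.
; Hits ignore the blaster and sibling lasers; otherwise the projectile is destroyed.
; HitFunction grants bullet-time points outside bullet time, rescales damage by distance beyond a threshold, and adds an aiming bonus.
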(event OnComponentHit(BulletCollision)
  (params (HitComponent :type Primitive%20Component%20Object%20Reference) (OtherActor :type Actor%20Object%20Reference) (OtherComp :type Primitive%20Component%20Object%20Reference) (NormalImpulse :type Vector :default "0, 0, 0") (Hit :type Hit%20Result%20Structure%20%28by%20ref%29))
  (Utilities|Casting|CastToBlaster_BP OtherActor
    (:CastFailed
      (Utilities|Casting|CastToBP_ShotGunLaser OtherActor
        (:CastFailed
          (bind _asdestroy_envionment (Utilities|Casting|CastToDestroyEnvionment OtherActor)
            (:then
              (Actor|DestroyActor _asdestroy_envionment))
            (:CastFailed
              _))
          (bind _asbomb_enemy (Utilities|Casting|CastToBombEnemy OtherActor)
            (:then
              (CallFunction|HitFunction 0 _asbomb_enemy))
            (:CastFailed
              _))
          (bind _asdistant_enemy (Utilities|Casting|CastToDistantEnemy OtherActor)
            (:then
              (CallFunction|HitFunction _asdistant_enemy))
            (:CastFailed
              _))
          (Actor|DestroyActor))))))

(event EventBeginPlay
  (Variables|Default|Setorigin (Transformation|GetWorldLocation (Variables|Default|GetBulletCollision)))
  (Utilities|FlowControl|Delay (/ (Variables|Default|GetrangeMax) (Variables|/Script/Engine.ProjectileMovementComponent|GetInitialSpeed (Variables|Default|GetProjectileMovement))))
  (Actor|DestroyActor))

(event EventTick
  (params (DeltaSeconds :type Float%20%28single-precision%29))
  (Class|ParticleSystemComponent|SetBeamSourcePoint (Variables|Default|GetP_Laser) 0 (Transformation|GetWorldLocation (Variables|Default|GetBulletCollision)))
  (Class|ParticleSystemComponent|SetBeamEndPoint (Variables|Default|GetP_Laser) 0 (Transformation|GetWorldLocation (Variables|Default|GetScene))))

(fn ConstructionScript)

(fn NormalDamage20
  (bind _outactors (Actor|GetAllActorsOfClass "/Game/Blueprints/AI/BombEnemy.BombEnemy_C"))
  (Variables|/Game/Blueprints/AI/BombEnemy.BombEnemy_C|SetHealth (Utilities|Array|Get(acopy) _outactors) (- (Variables|/Game/Blueprints/AI/BombEnemy.BombEnemy_C|GetHealth (Utilities|Array|Get(acopy) _outactors)) 1.5e+02)))

(fn HitFunction
  (params (distantEnnemis :type Distant%20Enemy%20Object%20Reference) (bombEnnemis :type Bomb%20Enemy%20Object%20Reference))
  (bind _origin (Variables|Default|Getorigin))
  (bind _bulletcollision (Variables|Default|GetBulletCollision))
  (bind _returnvalue (Transformation|GetWorldLocation _bulletcollision))
  (bind _returnvalue_2 (Math|Vector|Distance(Vector) _origin _returnvalue))
  (bind _ashunter_bp (Utilities|Casting|CastToHunter_BP (Game|Player|GetPlayerPawn 0)))
  (if (Variables|/Game/Blueprints/Hunter_BP.Hunter_BP_C|GetBulletTime _ashunter_bp)
    _
    (else
      (Default|BulletTimeGain _ashunter_bp (Variables|Default|GetBulletTimePoint))))
  (if (>= _returnvalue_2 (* (Variables|Default|GetdamageRangeInMeter) 1e+02))
    (LocalVariables|SetdamageTaken (* (Variables|Default|Getdamage) (- (/ _returnvalue_2 (Variables|Default|GetrangeMax)) 0.5)))
    (else
      (LocalVariables|SetdamageTaken (Variables|Default|Getdamage))))
  (if (Utilities|IsValid distantEnnemis)
    (if (Variables|/Game/Blueprints/Hunter_BP.Hunter_BP_C|GetIsAiming _ashunter_bp)
      (Default|DamageTaken distantEnnemis (+ (LocalVariables|GetdamageTaken) 5.0))
      (else
        (Default|DamageTaken distantEnnemis (LocalVariables|GetdamageTaken))))
    (elif (Utilities|IsValid bombEnnemis)
      (if (Variables|/Game/Blueprints/Hunter_BP.Hunter_BP_C|GetIsAiming _ashunter_bp)
        (Default|DamageTaken bombEnnemis (+ (LocalVariables|GetdamageTaken) 5.0))
        (else
          (Default|DamageTaken bombEnnemis (LocalVariables|GetdamageTaken)))))))