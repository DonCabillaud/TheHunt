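; Player blaster that fires normal, shotgun or bouncing lasers according to ShootMode.
; Fire traces from Hunter_BP's follow camera and spawns projectiles at the muzzle aimed at that point, with random shotgun spread, muzzle effects and sound.
; Tick spawns a test bouncing laser every frame while the hunter aims in bounce mode, sharing the bounce limit.
; Tick also recolors the blaster material in three tiers from the hunter's Overheat.
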(event EventTick
  (params (DeltaSeconds :type Float%20%28single-precision%29))
  (bind _spawnbullet (Variables|Default|GetspawnBullet))
  (bind _returnvalue (Transformation|GetWorldTransform _spawnbullet))
  (Utilities|FlowControl|Sequence
    (:then_0
      (bind _ashunter_bp (Utilities|Casting|CastToHunter_BP (Game|GetPlayerCharacter 0)))
      (if (Variables|/Game/Blueprints/Hunter_BP.Hunter_BP_C|GetBounceModeActive _ashunter_bp)
        (if (Variables|/Game/Blueprints/Hunter_BP.Hunter_BP_C|GetIsAiming _ashunter_bp)
          (bind _outhit (Collision|LineTraceByChannel (Transformation|GetWorldLocation (Variables|/Game/Blueprints/Hunter_BP.Hunter_BP_C|GetFollowCamera _ashunter_bp)) (+ (Transformation|GetWorldLocation (Variables|/Game/Blueprints/Hunter_BP.Hunter_BP_C|GetFollowCamera _ashunter_bp)) (* (Math|Vector|GetForwardVector (Transformation|GetWorldRotation (Variables|/Game/Blueprints/Hunter_BP.Hunter_BP_C|GetFollowCamera _ashunter_bp))) 2.5e+03)) "TraceTypeQuery1" false 0 "None" true "(R=0.000000,G=0.091400,B=1.000000,A=1.000000)"))
          ;[1 1 1] Boucing shot
          (bind _returnvalue_2 (Game|SpawnActorfromClass "/Game/Blueprints/TirsModes/BP_BouncingLaserrTest.BP_BouncingLaserrTest_C" (Math|Transform|MakeTransform (.location _returnvalue) (Math|Rotator|FindLookatRotation (.location _returnvalue) (Math|Vector|SelectVector (.ImpactPoint (Collision|BreakHitResult _outhit)) (.TraceEnd (Collision|BreakHitResult _outhit)) (.bBlockingHit (Collision|BreakHitResult _outhit)))) "0.100000,0.100000,0.100000") "Undefined" 0 0))
          (Variables|/Game/Blueprints/TirsModes/BP_BouncingLaserrTest.BP_BouncingLaserrTest_C|SetmaxBoucing _returnvalue_2 (Variables|Default|GetnbBounceOnBouncingShoot)))))
    (:then_1
      (bind _ashunter_bp_2 (Utilities|Casting|CastToHunter_BP (Game|GetPlayerCharacter 0)))
      (if (and (>= (Variables|/Game/Blueprints/Hunter_BP.Hunter_BP_C|GetOverheat _ashunter_bp_2) 0.0) (< (Variables|/Game/Blueprints/Hunter_BP.Hunter_BP_C|GetOverheat _ashunter_bp_2) 5.0))
        (Rendering|Material|SetVectorParameterValueonMaterials (Variables|Default|GetBlasterdeSubstitution) "Overheat" "0.180000,0.180000,0.180000")
        (elif (and (>= (Variables|/Game/Blueprints/Hunter_BP.Hunter_BP_C|GetOverheat _ashunter_bp_2) 5.0) (< (Variables|/Game/Blueprints/Hunter_BP.Hunter_BP_C|GetOverheat _ashunter_bp_2) 9.0))
          (Rendering|Material|SetVectorParameterValueonMaterials (Variables|Default|GetBlasterdeSubstitution) "Overheat" "0.600000,0.600000,0.180000")
          (elif (and (>= (Variables|/Game/Blueprints/Hunter_BP.Hunter_BP_C|GetOverheat _ashunter_bp_2) 9.0) (<= (Variables|/Game/Blueprints/Hunter_BP.Hunter_BP_C|GetOverheat _ashunter_bp_2) 1e+01))
            (Rendering|Material|SetVectorParameterValueonMaterials (Variables|Default|GetBlasterdeSubstitution) "Overheat" "1.000000, 0,0.180000")))))))

(fn ConstructionScript)

(fn Fire
  (bind _spawnbullet (Variables|Default|GetspawnBullet))
  (bind _spawnbullet_2 (Variables|Default|GetspawnBullet))
  (bind _spawnbullet_3 (Variables|Default|GetspawnBullet))
  (bind _shotgunprecision (Variables|Default|GetshotgunPrecision))
  (bind _spawnbullet_4 (Variables|Default|GetspawnBullet))
  (bind _returnvalue (Transformation|GetWorldTransform _spawnbullet))
  (bind _returnvalue_2 (Transformation|GetWorldLocation _spawnbullet_3))
  (bind _returnvalue_3 (Transformation|GetWorldLocation _spawnbullet_4))
  (bind _returnvalue_4 (Transformation|GetWorldLocation _spawnbullet_2))
  ;[1 1 1] Orientation des projectiles
  (bind _ashunter_bp (Utilities|Casting|CastToHunter_BP (Game|GetPlayerCharacter 0)))
  (bind _outhit (Collision|LineTraceByChannel (Transformation|GetWorldLocation (Variables|/Game/Blueprints/Hunter_BP.Hunter_BP_C|GetFollowCamera _ashunter_bp)) (+ (Transformation|GetWorldLocation (Variables|/Game/Blueprints/Hunter_BP.Hunter_BP_C|GetFollowCamera _ashunter_bp)) (* (Math|Vector|GetForwardVector (Transformation|GetWorldRotation (Variables|/Game/Blueprints/Hunter_BP.Hunter_BP_C|GetFollowCamera _ashunter_bp))) 2.5e+03)) "TraceTypeQuery1" false 0 "None" true "(R=0.000000,G=0.091400,B=1.000000,A=1.000000)"))
  ;[1 1 1] Normal Shot
  (if (== (Variables|Default|GetshootMode) 0)
    (Effects|SpawnEmitteratLocation "/Game/FXVarietyPack/Particles/P_ky_shotShockwave.P_ky_shotShockwave" _returnvalue_4 (Transformation|GetWorldRotation _spawnbullet_2) "0.200000,0.200000,0.200000")
    (Game|SpawnActorfromClass "/Game/Blueprints/TirsModes/BP_NormalLaser.BP_NormalLaser_C" (Math|Transform|MakeTransform (.location _returnvalue) (Math|Rotator|FindLookatRotation (.location _returnvalue) (Math|Vector|SelectVector (.ImpactPoint (Collision|BreakHitResult _outhit)) (.TraceEnd (Collision|BreakHitResult _outhit)) (.bBlockingHit (Collision|BreakHitResult _outhit)))) "0.100000,0.100000,0.100000") "Undefined" 0 0)
    (Audio|PlaySoundatLocation "/Game/Sounds/SFX/Laser_Shot.Laser_Shot" _returnvalue_4 "0, 0, 0" 1.0 1.0 0.0 0 0 0)
    (else
      ;[1 1 1] ShotGun shot
      (if (== (Variables|Default|GetshootMode) 1)
        ;;[0.4664 0.5434 1] SpawnMuzzleFlash
        (Effects|SpawnEmitteratLocation "/Game/FXVarietyPack/Particles/P_ky_shotShockwave.P_ky_shotShockwave" _returnvalue_3 (Transformation|GetWorldRotation _spawnbullet_4) "0.400000,0.400000,0.400000")
        (for _index (range 0 (Variables|Default|GetnbShotGunProjectile))
          (Game|SpawnActorfromClass "/Game/Blueprints/TirsModes/BP_ShotGunLaser.BP_ShotGunLaser_C" (Math|Transform|MakeTransform (.location _returnvalue) (Math|Rotator|MakeRotator (.Roll (Math|Rotator|BreakRotator (Math|Rotator|FindLookatRotation (.location _returnvalue) (Math|Vector|SelectVector (.ImpactPoint (Collision|BreakHitResult _outhit)) (.TraceEnd (Collision|BreakHitResult _outhit)) (.bBlockingHit (Collision|BreakHitResult _outhit)))))) (+ (* (- (Math|Random|RandomFloat) 0.5) _shotgunprecision) (.Pitch (Math|Rotator|BreakRotator (Math|Rotator|FindLookatRotation (.location _returnvalue) (Math|Vector|SelectVector (.ImpactPoint (Collision|BreakHitResult _outhit)) (.TraceEnd (Collision|BreakHitResult _outhit)) (.bBlockingHit (Collision|BreakHitResult _outhit))))))) (+ (.Yaw (Math|Rotator|BreakRotator (Math|Rotator|FindLookatRotation (.location _returnvalue) (Math|Vector|SelectVector (.ImpactPoint (Collision|BreakHitResult _outhit)) (.TraceEnd (Collision|BreakHitResult _outhit)) (.bBlockingHit (Collision|BreakHitResult _outhit)))))) (* (- (Math|Random|RandomFloat) 0.5) _shotgunprecision))) "0.100000,0.100000,0.100000") "Undefined" 0 0)
          (Audio|PlaySoundatLocation "/Game/Sounds/SFX/Laser_Shot.Laser_Shot" _returnvalue_3 "0, 0, 0" 1.0 0.2 0.0 0 0 0))
        (else
          ;[1 1 1] Boucing shot
          (if (== (Variables|Default|GetshootMode) 2)
            (Effects|SpawnEmitteratLocation "/Game/FXVarietyPack/Particles/P_ky_shotShockwave.P_ky_shotShockwave" _returnvalue_2 (Transformation|GetWorldRotation _spawnbullet_3) "0.300000,0.300000,0.300000")
            (bind _returnvalue_5 (Game|SpawnActorfromClass "/Game/Blueprints/TirsModes/BP_BouncingLaserr.BP_BouncingLaserr_C" (Math|Transform|MakeTransform (.location _returnvalue) (Math|Rotator|FindLookatRotation (.location _returnvalue) (Math|Vector|SelectVector (.ImpactPoint (Collision|BreakHitResult _outhit)) (.TraceEnd (Collision|BreakHitResult _outhit)) (.bBlockingHit (Collision|BreakHitResult _outhit)))) "0.100000,0.100000,0.100000") "Undefined" 0 0))
            (Audio|PlaySoundatLocation "/Game/Sounds/SFX/bounce_laser_.bounce_laser_" _returnvalue_2 "0, 0, 0" 1.0 1.0 0.0 0 0 0)
            (Variables|/Game/Blueprints/TirsModes/BP_BouncingLaserr.BP_BouncingLaserr_C|SetmaxBoucing _returnvalue_5 (Variables|Default|GetnbBounceOnBouncingShoot))))))))