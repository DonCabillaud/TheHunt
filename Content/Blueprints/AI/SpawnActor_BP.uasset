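; One-shot trigger volume that spawns AI robot enemies when a Hunter_BP enters it.
; Each valid actor in the Enemy array marks a spawn transform and is destroyed after its robot spawns with AI_BT and an arrival sound.
; The parallel RobotType bool array selects BombEnemy when true, falling back to DistantEnemy when false or missing.
; The spawner destroys itself once the loop finishes.
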(event OnComponentBeginOverlap(SpawnTrigger)
  (params (OverlappedComponent :type Primitive%20Component%20Object%20Reference) (OtherActor :type Actor%20Object%20Reference) (OtherComp :type Primitive%20Component%20Object%20Reference) (OtherBodyIndex :type Integer) (bFromSweep :type Boolean) (SweepResult :type Hit%20Result%20Structure%20%28by%20ref%29))
  (bind _robottype (Variables|Default|GetRobotType))
  (Utilities|Casting|CastToHunter_BP OtherActor)
  (Utilities|FlowControl|DoOnce false
    (:Completed
      (for (_array_element _array_index) (Variables|Default|GetEnemy)
        (if (Utilities|IsValid _array_element)
          (if (> _array_index (Utilities|Array|LastIndex _robottype))
            (AI|SpawnAIFromClass "/Game/Blueprints/AI/DistantEnemy.DistantEnemy_C" "/Game/Blueprints/AI/AI_BT.AI_BT" (.location (Transformation|GetWorldTransform (Variables|/Script/Engine.Actor|GetRootComponent _array_element))) (.rotation (Transformation|GetWorldTransform (Variables|/Script/Engine.Actor|GetRootComponent _array_element))) false 0 :!label _label)
            (elif (Utilities|Array|Get(acopy) _robottype _array_index)
              (AI|SpawnAIFromClass "/Game/Blueprints/AI/BombEnemy.BombEnemy_C" "/Game/Blueprints/AI/AI_BT.AI_BT" (.location (Transformation|GetWorldTransform (Variables|/Script/Engine.Actor|GetRootComponent _array_element))) (.rotation (Transformation|GetWorldTransform (Variables|/Script/Engine.Actor|GetRootComponent _array_element))) false 0)
              (else
                (goto _label))))
          (Audio|PlaySoundatLocation "/Game/Sounds/SFX/drone_arrive.drone_arrive" (.location (Transformation|GetWorldTransform (Variables|/Script/Engine.Actor|GetRootComponent _array_element))) "0, 0, 0" 0.15 1.0 0.0 0 0 0)
          (Actor|DestroyActor _array_element)))
      (Actor|DestroyActor))))

(fn ConstructionScript)