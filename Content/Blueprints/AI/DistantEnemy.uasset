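; Ranged enemy AI that chases the Hunter player, fires lasers and is protected by an armor shield.
; Tick updates range flags, turns the capsule toward the player and uses AIMoveTo to approach until inside minimum distance.
; Shoot re-calls itself after a delay, spawning aimed BP_EnnemiLaser projectiles while the player stays in range.
; DamageTaken drains armor before health and destroys the actor at zero health, while Tick recolors or hides the shield by remaining armor.
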(event Custom|shoot
  (bind _spawn_projectile (Variables|Default|Getspawn%20projectile))
  (bind _returnvalue (Transformation|GetWorldLocation _spawn_projectile))
  ;[1 1 1] Shoot
  (if (Variables|Default|GetisInRange)
    (Variables|Default|SetisShooting true)
    (Utilities|FlowControl|Delay 1.0)
    (bind _ashunter_bp (Utilities|Casting|CastToHunter_BP (Game|Player|GetPlayerPawn 0)))
    (bind _returnvalue_2 (Game|SpawnActorfromClass "/Game/Blueprints/TirsModes/BP_EnnemiLaser.BP_EnnemiLaser_C" (Math|Transform|MakeTransform _returnvalue (Math|Rotator|FindLookatRotation _returnvalue (Transformation|GetWorldLocation (Variables|/Script/Engine.Character|GetCapsuleComponent _ashunter_bp))) "0.100000,0.100000,0.100000") "Undefined" 0 0))
    (Variables|/Script/Engine.ProjectileMovementComponent|SetInitialSpeed (Variables|/Game/Blueprints/TirsModes/BP_EnnemiLaser.BP_EnnemiLaser_C|GetProjectileMovement _returnvalue_2) 1e+03)
    (Variables|/Script/Engine.ProjectileMovementComponent|SetMaxSpeed (Variables|/Game/Blueprints/TirsModes/BP_EnnemiLaser.BP_EnnemiLaser_C|GetProjectileMovement _returnvalue_2) 1e+03)
    (CallFunction|Shoot)
    (else
      (Variables|Default|SetisShooting false))))

(event EventTick
  (params (DeltaSeconds :type Float%20%28single-precision%29))
  (bind _returnvalue (Game|Player|GetPlayerPawn 0))
  (bind _self self)
  (bind _capsulecomponent (Variables|Collision|GetCapsuleComponent))
  (bind _armorpoint (Variables|Default|GetArmorPoint))
  (bind _armorpoint_2 (Variables|Default|GetArmorPoint))
  (bind _armorpoint_3 (Variables|Default|GetArmorPoint))
  (bind _capsulecomponent_2 (Variables|Collision|GetCapsuleComponent))
  (bind _shield (Variables|Default|GetShield))
  (bind _returnvalue_2 (Transformation|GetActorLocation _returnvalue))
  (bind _returnvalue_3 (Transformation|GetWorldLocation _capsulecomponent_2))
  (bind _relativerotation (Variables|/Script/Engine.SceneComponent|GetRelativeRotation _capsulecomponent))
  (bind _returnvalue_4 (Math|Vector|Distance(Vector) _returnvalue_3 _returnvalue_2))
  (Utilities|FlowControl|Sequence
    (:then_0
      (if (< _returnvalue_4 (Variables|Default|GetShootRangeMax))
        (Variables|Default|SetisInRange true)
        (else
          (Variables|Default|SetisInRange false)))
      (if (> _returnvalue_4 (Variables|Default|GetMoveRangeMin))
        (Variables|Default|SetisMoving true)
        (else
          (Variables|Default|SetisMoving false)))
      ;[1 1 1] target
      (bind _ashunter_bp (Utilities|Casting|CastToHunter_BP (Game|Player|GetPlayerPawn 0)))
      (Transformation|SetRelativeRotation _capsulecomponent (Math|Rotator|MakeRotator (.roll _relativerotation) (.pitch _relativerotation) (- (.yaw (Math|Rotator|FindLookatRotation (Variables|/Script/Engine.SceneComponent|GetRelativeLocation _capsulecomponent) (Variables|/Script/Engine.SceneComponent|GetRelativeLocation (Variables|/Script/Engine.Character|GetCapsuleComponent _ashunter_bp)))) 9e+01)) false false)
      ;[1 1 1] movement
      (if (Variables|Default|GetisMoving)
        (AI|AIMoveTo _self "0, 0, 0" _ashunter_bp 5.0 false
          (:then
            _))
        (else
          (AI|AIMoveTo _self "0, 0, 0" _self 5.0 false
            (:then
              _))))
      (if (not (Variables|Default|GetisShooting))
        (CallFunction|Shoot)))
    (:then_1
      ;[1 1 1] Shield
      (if (and (> _armorpoint 25.0) (<= _armorpoint 5e+01))
        (Rendering|Material|SetVectorParameterValueonMaterials _shield "Shield" "0,0.385502,1.000000")
        (elif (and (> _armorpoint_2 15.0) (<= _armorpoint_2 35.0))
          (Rendering|Material|SetVectorParameterValueonMaterials _shield "Shield" "1.000000,0.949909,0.006095")
          (elif (and (> _armorpoint_3 0.0) (<= _armorpoint_3 15.0))
            (Rendering|Material|SetVectorParameterValueonMaterials _shield "Shield" "1.000000,0.000000,0.000000")
            (elif (<= (Variables|Default|GetArmorPoint) 0.0)
              (Rendering|SetVisibility (Variables|Default|GetShield) false false))))))))

(fn ConstructionScript)

(fn DamageTaken
  (params (damage :type Float%20%28single-precision%29))
  (Variables|Default|SetisPursuit true)
  (if (<= (Variables|Default|GetArmorPoint) 0.0)
    (Variables|Default|SetHealthPoint (- (Variables|Default|GetHealthPoint) damage))
    (if (<= (Variables|Default|GetHealthPoint) 0.0) :!label _label
      (Actor|DestroyActor))
    (elif (< (Variables|Default|GetArmorPoint) damage)
      (Variables|Default|SetHealthPoint (- (Variables|Default|GetHealthPoint) (- damage (Variables|Default|GetArmorPoint))))
      (Variables|Default|SetArmorPoint 0.0)
      (goto _label)
      (else
        (Variables|Default|SetArmorPoint (- (Variables|Default|GetArmorPoint) damage))))))