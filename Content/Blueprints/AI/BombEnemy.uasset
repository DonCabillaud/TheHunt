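; BombEnemy is a suicide-bomber AI enemy that explodes when the player reaches it or its health runs out.
; Either trigger stops it, shows the explosion indicator and plays the Grossi timeline as a fuse.
; When the timeline finishes, it spawns an explosion emitter, damages the player if flagged in range, and destroys itself.
; The StopCollision overlap sets and clears that IsInExplosion flag on Hunter_BP.
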(event OnComponentBeginOverlap(StopCollision)
  (params (OverlappedComponent :type Primitive%20Component%20Object%20Reference) (OtherActor :type Actor%20Object%20Reference) (OtherComp :type Primitive%20Component%20Object%20Reference) (OtherBodyIndex :type Integer) (bFromSweep :type Boolean) (SweepResult :type Hit%20Result%20Structure%20%28by%20ref%29))
  (bind _charactermovement (Variables|Character|GetCharacterMovement))
  (bind _explosion (Variables|Default|GetExplosion))
  (bind _ashunter_bp (Utilities|Casting|CastToHunter_BP OtherActor))
  (Variables|/Game/Blueprints/Hunter_BP.Hunter_BP_C|SetIsInExplosion _ashunter_bp true)
  (Components|Movement|StopMovementImmediately _charactermovement)
  (Variables|/Script/Engine.CharacterMovementComponent|SetMaxWalkSpeed _charactermovement 0.0)
  (Rendering|SetVisibility _explosion true false)
  (Timeline|grossi Play
    (:Finished
      (Rendering|SetVisibility _explosion false false)
      (Effects|SpawnEmitteratLocation "/Game/StarterContent/Particles/P_Explosion.P_Explosion" (Transformation|GetActorLocation) "0, 0, 0" "20.000000,20.000000,20.000000")
      (bind _ashunter_bp_2 (Utilities|Casting|CastToHunter_BP (Game|GetPlayerCharacter 0)))
      (if (Variables|/Game/Blueprints/Hunter_BP.Hunter_BP_C|GetIsInExplosion _ashunter_bp_2)
        (CallFunction|ExplosionDamage))
      (Actor|DestroyActor))))

(event OnComponentEndOverlap(StopCollision)
  (params (OverlappedComponent :type Primitive%20Component%20Object%20Reference) (OtherActor :type Actor%20Object%20Reference) (OtherComp :type Primitive%20Component%20Object%20Reference) (OtherBodyIndex :type Integer))
  (bind _ashunter_bp (Utilities|Casting|CastToHunter_BP OtherActor))
  (Variables|/Game/Blueprints/Hunter_BP.Hunter_BP_C|SetIsInExplosion _ashunter_bp false))

(event EventBeginPlay
  ;[1 1 1] hide explosion indicator area
  (Rendering|SetVisibility (Variables|Default|GetExplosion) false false))

(event EventTick
  (params (DeltaSeconds :type Float%20%28single-precision%29))
  (bind _explosion (Variables|Default|GetExplosion))
  (if (<= (Variables|Default|GetHealth) 0.0)
    (Variables|/Script/Engine.CharacterMovementComponent|SetMaxWalkSpeed (Variables|Character|GetCharacterMovement) 0.0)
    (Rendering|SetVisibility _explosion true false)
    (Timeline|grossi Play
      (:Finished
        (Rendering|SetVisibility _explosion false false)
        (Effects|SpawnEmitteratLocation "/Game/StarterContent/Particles/P_Explosion.P_Explosion" (Transformation|GetActorLocation) "0, 0, 0" "20.000000,20.000000,20.000000")
        (bind _ashunter_bp (Utilities|Casting|CastToHunter_BP (Game|GetPlayerCharacter 0)))
        (if (Variables|/Game/Blueprints/Hunter_BP.Hunter_BP_C|GetIsInExplosion _ashunter_bp)
          (CallFunction|ExplosionDamage))
        (Actor|DestroyActor)))))

(fn ConstructionScript)

(fn ExplosionDamage
  (bind _ashunter_bp (Utilities|Casting|CastToHunter_BP (Game|GetPlayerCharacter 0)))
  (Default|DamageTaken _ashunter_bp (Variables|Default|GetExplosionDamage20)))

(fn DamageTaken
  (params (Damage :type Float%20%28single-precision%29))
  (Variables|Default|SetHealth (- (Variables|Default|GetHealth) Damage)))