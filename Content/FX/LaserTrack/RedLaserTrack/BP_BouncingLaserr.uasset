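; Bouncing laser projectile that damages enemies, with a beam particle drawn each tick between its collision component and scene component.
; Hits, ignoring the blaster and other lasers, increment a bounce count until the maximum destroys it; a timer also destroys it.
; Damage grows per bounce, but chained casts only reach the DistantEnemy check after BombEnemy succeeds.
; NormalDamage20, uncalled here, subtracts fixed health from the first BombEnemy found.
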(event OnComponentHit(BulletCollision)
  (params (HitComponent :type Primitive%20Component%20Object%20Reference) (OtherActor :type Actor%20Object%20Reference) (OtherComp :type Primitive%20Component%20Object%20Reference) (NormalImpulse :type Vector :default "0, 0, 0") (Hit :type Hit%20Result%20Structure%20%28by%20ref%29))
  (bind _damage (Variables|Default|GetDamage))
  (bind _damageadd (Variables|Default|GetdamageAdd))
  (bind _currentboucing (Variables|Default|GetcurrentBoucing))
  (bind _currentboucing_2 (Variables|Default|GetcurrentBoucing))
  (bind _returnvalue (* _currentboucing_2 _damageadd))
  (bind _returnvalue_2 (+ _damage _returnvalue))
  (Utilities|Casting|CastToBlaster_BP OtherActor
    (:CastFailed
      (Utilities|Casting|CastToBP_BouncingLaserr OtherActor
        (:CastFailed
          (Utilities|FlowControl|Sequence
            (:then_0
              (bind _asbomb_enemy (Utilities|Casting|CastToBombEnemy OtherActor))
              (Default|DamageTaken _asbomb_enemy _returnvalue_2)
              (bind _asdistant_enemy (Utilities|Casting|CastToDistantEnemy OtherActor))
              (Default|DamageTaken _asdistant_enemy _returnvalue_2)
              (Actor|DestroyActor :!label _label))
            (:then_1
              (if (== _currentboucing (Variables|Default|GetmaxBoucing))
                (goto _label)
                (else
                  (Math|Integer|IncrementInt _currentboucing))))))))))

(event EventBeginPlay
  (Variables|Default|SetcurrentBoucing 0)
  (Utilities|FlowControl|Delay 1e+01)
  (Actor|DestroyActor))

(event EventTick
  (params (DeltaSeconds :type Float%20%28single-precision%29))
  (Class|ParticleSystemComponent|SetBeamSourcePoint (Variables|Default|GetP_Laser) 0 (Transformation|GetWorldLocation (Variables|Default|GetBulletCollision)))
  (Class|ParticleSystemComponent|SetBeamEndPoint (Variables|Default|GetP_Laser) 0 (Transformation|GetWorldLocation (Variables|Default|GetScene))))

(fn ConstructionScript)

(fn NormalDamage20
  (bind _outactors (Actor|GetAllActorsOfClass "/Game/Blueprints/AI/BombEnemy.BombEnemy_C"))
  (Variables|/Game/Blueprints/AI/BombEnemy.BombEnemy_C|SetHealth (Utilities|Array|Get(acopy) _outactors) (- (Variables|/Game/Blueprints/AI/BombEnemy.BombEnemy_C|GetHealth (Utilities|Array|Get(acopy) _outactors)) 1.5e+02)))